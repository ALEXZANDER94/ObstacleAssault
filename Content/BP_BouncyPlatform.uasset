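; Bouncy cloud platform that launches the player's third-person character when it overlaps the collision component.
; The velocity-change impulse follows the inverted sweep normal, scaled from ImpulseVelocity.
; It is strongest when the character is not falling, and while falling it is reduced sharply for steeply downward impact normals.
; Each bounce replays a timeline that lerps the scale of the cloud meshes as visual feedback.
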(event OnComponentBeginOverlap(Collision)
  (params (OverlappedComponent :type Primitive%20Component%20Object%20Reference) (OtherActor :type Actor%20Object%20Reference) (OtherComp :type Primitive%20Component%20Object%20Reference) (OtherBodyIndex :type Integer) (bFromSweep :type Boolean) (SweepResult :type Hit%20Result%20Structure%20%28by%20ref%29))
  (bind _returnvalue (Game|Player|GetPlayerPawn 0))
  (bind (_bblockinghit _binitialoverlap _time _distance _location _impactpoint _normal _impactnormal) (Collision|BreakHitResult SweepResult))
  (bind _impulsevelocity (Variables|Default|GetImpulseVelocity))
  (if (== OtherActor _returnvalue)
    (bind _asbp_third_person_character (Utilities|Casting|CastToBP_ThirdPersonCharacter _returnvalue))
    (if (AI|Components|NavMovement|IsFalling (Variables|/Script/Engine.Character|GetCharacterMovement _asbp_third_person_character))
      (if (<= (.Z (Math|Vector|BreakVector _impactnormal)) -0.5)
        (Physics|AddImpulse (Variables|/Script/Engine.Character|GetCharacterMovement _asbp_third_person_character) (* _normal -1 (/ _impulsevelocity 5.0)) true)
        (else
          (Physics|AddImpulse (Variables|/Script/Engine.Character|GetCharacterMovement _asbp_third_person_character) (* _normal -1 _impulsevelocity) true)))
      (else
        (Physics|AddImpulse (Variables|/Script/Engine.Character|GetCharacterMovement _asbp_third_person_character) (* _normal -1 (* _impulsevelocity 2.5)) true)))
    (CallFunction|BounceEffect)))

(event Custom|BounceEffect
  (bind _f_bounce (Timeline|TL_Bounc PlayFromStart)
    (:Update
      (Transformation|SetRelativeScale3D (Variables|Default|GetSM_Cloud_B2) (Math|Vector|Lerp(Vector) "0.050000,0.050000,0.100000" "0.075000,0.075000,0.125000" _f_bounce))
      (Transformation|SetRelativeScale3D (Variables|Default|GetSM_Cloud_B1) (Math|Vector|Lerp(Vector) "0.050000,0.050000,0.100000" "0.075000,0.075000,0.125000" _f_bounce))
      (Transformation|SetRelativeScale3D (Variables|Default|GetSM_Cloud_B) (Math|Vector|Lerp(Vector) "0.050000,0.050000,0.100000" "0.075000,0.075000,0.125000" _f_bounce))
      (Transformation|SetRelativeScale3D (Variables|Default|GetSM_Cloud_B3) (Math|Vector|Lerp(Vector) "0.050000,0.050000,0.100000" "0.075000,0.075000,0.125000" _f_bounce))
      (Transformation|SetRelativeScale3D (Variables|Default|GetSM_Cloud_B4) (Math|Vector|Lerp(Vector) "0.050000,0.050000,0.100000" "0.075000,0.075000,0.125000" _f_bounce))
      (Transformation|SetRelativeScale3D (Variables|Default|GetSM_Cloud_B5) (Math|Vector|Lerp(Vector) "0.050000,0.050000,0.100000" "0.075000,0.075000,0.125000" _f_bounce))
      (Transformation|SetRelativeScale3D (Variables|Default|GetSM_Cloud_B6) (Math|Vector|Lerp(Vector) "0.050000,0.050000,0.100000" "0.075000,0.075000,0.125000" _f_bounce)))))

(event EventBeginPlay)

(event EventTick
  (params (DeltaSeconds :type Float%20%28single-precision%29)))

(fn ConstructionScript)